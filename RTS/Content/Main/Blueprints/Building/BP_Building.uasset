(event `self.ReceiveBeginPlay`
  (`PrimitiveComponent.SetMaterial` (`self.Cube`) 0 "/Game/Main/Matérials/ValidConstruction/M_Valid.M_Valid"))

(event `self.Cube.OnComponentBeginOverlap`
  (params (OverlappedComponent :type "PrimitiveComponent Object Reference") (OtherActor :type "Actor Object Reference") (OtherComp :type "PrimitiveComponent Object Reference") (OtherBodyIndex :type Integer) (bFromSweep :type Boolean) (SweepResult :type "HitResult Structure (by ref)"))
  (if (not (`self.IsConstructed`))
    (`PrimitiveComponent.SetMaterial` (`self.Cube`) 0 "/Game/Main/Matérials/ValidConstruction/M_NotValid.M_NotValid")))

(event `self.Cube.OnComponentEndOverlap`
  (params (OverlappedComponent :type "PrimitiveComponent Object Reference") (OtherActor :type "Actor Object Reference") (OtherComp :type "PrimitiveComponent Object Reference") (OtherBodyIndex :type Integer))
  (if (not (`self.IsConstructed`))
    (`PrimitiveComponent.SetMaterial` (`self.Cube`) 0 "/Game/Main/Matérials/ValidConstruction/M_Valid.M_Valid")))

(event `/Game/Main/Blueprints/Interface/BPI_Selectable.Attacked`
  (params (Agressor :type "Actor Object Reference") (Damage :type Integer))
  (bind _output_get (set `self.Life` (- (`self.Life`) Damage)))
  (if (<= _output_get 0)
    (`KismetSystemLibrary.PrintText` (`|FormatText` "{a} killed {b}" Agressor self))
    (`self.K2_DestroyActor`)))

(fn `Build`
  (returns (CanBuild :type Boolean))
  (if (`KismetArrayLibrary.Array_IsEmpty` (`PrimitiveComponent.GetOverlappingActors` (`self.Cube`) "/Script/Engine.Actor"))
    (`PrimitiveComponent.SetCollisionProfileName` (`self.Cube`) "BuildingCollision" true)
    (`PrimitiveComponent.SetMaterial` (`self.Cube`) 0 "/Game/Main/Matérials/ValidConstruction/M_Constructed.M_Constructed")
    (set `self.IsConstructed` true)
    (return true)
    (else
      (return false))))

(fn `GetTeamIndex`
  (returns (TeamIndex :type Byte))
  (return (`self.TeamIndex`)))

(fn `UserConstructionScript`)