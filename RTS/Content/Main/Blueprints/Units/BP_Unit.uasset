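; BP_Unit is a controller-driven combat unit with a team index, life, damage and a toggleable focus indicator.
; Attack sends damage to the target through a message call, throttled by a time-based five-second cooldown.
; When attacked, it keeps an aggressor reference, passes it to its controller as a target, and subtracts life.
; At zero life or below, it prints a kill message and destroys itself.
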(event `/Game/Main/Blueprints/Units/Interface/BPI_Unit.ToggleFocus`
  (params (bIsFocus :type Boolean))
  (`SceneComponent.SetVisibility` (`self.Focus`) bIsFocus false))

(event `/Game/Main/Blueprints/Units/Interface/BPI_Unit.Attack`
  (params (Target :type "Object Object Reference"))
  (if (< 5.0 (- (`GameplayStatics.GetTimeSeconds`) (`self.LastTime`)))
    (set `self.LastTime` (`GameplayStatics.GetTimeSeconds`))
    (message `/Game/Main/Blueprints/Interface/BPI_Selectable.Attacked` Target self (`self.Damage`))))

(event `/Game/Main/Blueprints/Interface/BPI_Selectable.Attacked`
  (params (Agressor :type "Actor Object Reference") (Damage :type Integer))
  (`/Engine/EditorBlueprintResources/StandardMacros.IsValid` (`self.Agressor`)
    (:`Is Valid`
      _)
    (:`Is Not Valid`
      (bind _output_get (set `self.Agressor` Agressor))))
  (message `/Game/Main/Blueprints/Units/AIController/Interface/BPI_UnitController.SetTarget` (`self.GetController`) _output_get)
  (bind _output_get_2 (set `self.Life` (- (`self.Life`) Damage)))
  (if (<= _output_get_2 0)
    (`KismetSystemLibrary.PrintText` (`|FormatText` "{a} killed {b}" Agressor self))
    (`self.K2_DestroyActor`)))

(fn `GetTeamIndex`
  (returns (TeamIndex :type Byte))
  (return (`self.TeamIndex`)))

(fn `UserConstructionScript`)