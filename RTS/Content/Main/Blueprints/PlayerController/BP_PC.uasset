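; RTS-style player controller that drives the camera pawn and commands an army of AI units.
; Enhanced Input moves and rotates the camera, while zoom blends between spring arm length and pitch, tilting at closest range.
; Clicking units adds their AI controllers to Army and enables the order mapping context; an empty click clears both.
; Held orders steer units toward the cursor, and release sends MoveTo with two-wide grid offsets.
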(event `self.ReceiveBeginPlay`
  (bind _asbp_player_pawn (cast `/Game/Main/Blueprints/Player/BP_PlayerPawn` (`GameplayStatics.GetPlayerPawn` 0)))
  (set `self.As BP Player Pawn` _asbp_player_pawn)
  (`EnhancedInputSubsystemInterface.AddMappingContext` (subsystem `EnhancedInputLocalPlayerSubsystem`) "/Game/Main/Blueprints/PlayerController/Inputs/IMC/Default/IMC_Default.IMC_Default" 0 (struct))
  (set `self.bShowMouseCursor` true))

(event `EnhancedInput|/Game/Main/Blueprints/PlayerController/Inputs/Inputs/Default/IA_Move`
  (params (ActionValue :type "Vector2D Structure") (ElapsedSeconds :type "Float (double-precision)") (TriggeredSeconds :type "Float (double-precision)") (InputAction :type "InputAction Object Reference" :default "/Game/Main/Blueprints/PlayerController/Inputs/Inputs/Default/IA_Move.IA_Move"))
  (bind _arrow (`/Game/Main/Blueprints/Player/BP_PlayerPawn.Arrow` (`self.As BP Player Pawn`)))
  ;[1 0.009101 0 0.5] Camera
  (:`Triggered`
    (`Pawn.AddMovementInput` (`self.As BP Player Pawn`) (`SceneComponent.GetRightVector` _arrow) ActionValue_X false)
    (`Pawn.AddMovementInput` (`self.As BP Player Pawn`) (`SceneComponent.GetForwardVector` _arrow) ActionValue_Y false)))

(event `EnhancedInput|/Game/Main/Blueprints/PlayerController/Inputs/Inputs/Default/IA_Rotate`
  (params (ActionValue :type "Float (double-precision)") (ElapsedSeconds :type "Float (double-precision)") (TriggeredSeconds :type "Float (double-precision)") (InputAction :type "InputAction Object Reference" :default "/Game/Main/Blueprints/PlayerController/Inputs/Inputs/Default/IA_Rotate.IA_Rotate"))
  ;[1 0.009101 0 0.5] Camera
  (:`Triggered`
    (`self.K2_AddActorLocalRotation` (`self.As BP Player Pawn`) (`KismetMathLibrary.MakeRotator` 0.0 0.0 ActionValue) false false)))

(event `EnhancedInput|/Game/Main/Blueprints/PlayerController/Inputs/Inputs/Default/IA_Zoom`
  (params (ActionValue :type "Float (double-precision)") (ElapsedSeconds :type "Float (double-precision)") (TriggeredSeconds :type "Float (double-precision)") (InputAction :type "InputAction Object Reference" :default "/Game/Main/Blueprints/PlayerController/Inputs/Inputs/Default/IA_Zoom.IA_Zoom"))
  (bind _springarm (`/Game/Main/Blueprints/Player/BP_PlayerPawn.SpringArm` (`self.As BP Player Pawn`)))
  (bind _springarm_2 (`/Game/Main/Blueprints/Player/BP_PlayerPawn.SpringArm` (`self.As BP Player Pawn`)))
  (bind _springarm_3 (`/Game/Main/Blueprints/Player/BP_PlayerPawn.SpringArm` (`self.As BP Player Pawn`)))
  (bind (_relativerotation_roll _relativerotation_pitch) (`KismetMathLibrary.BreakRotator` (`SceneComponent.RelativeRotation` _springarm)))
  (bind (_relativerotation_roll_2 _relativerotation_pitch_2) (`KismetMathLibrary.BreakRotator` (`SceneComponent.RelativeRotation` _springarm_2)))
  ;[1 0.009101 0 0.5] Camera
  (:`Triggered`
    (set `self.Zoom` (* ActionValue -1.0))
    (if (== (`SceneComponent.RelativeRotation` _springarm) (`KismetMathLibrary.MakeRotator` 0.0 (`self.ZoomMin`)) :`ErrorTolerance` 0.1)
      (if (and (== (`SpringArmComponent.TargetArmLength` (`/Game/Main/Blueprints/Player/BP_PlayerPawn.SpringArm` (`self.As BP Player Pawn`))) 700.0) (< (`self.Zoom`) 0.0))
        (`SceneComponent.K2_SetRelativeRotation` _springarm_2 (`KismetMathLibrary.MakeRotator` 0.0 (`KismetMathLibrary.FClamp` (+ _relativerotation_pitch_2 (* (* (`self.Zoom`) -1.0) 10.0)) (`self.ZoomMin`) (`self.ZoomMax`))) false false)
        (else
          (set `SpringArmComponent.TargetArmLength` (`KismetMathLibrary.FClamp` (+ (* (`self.Zoom`) 100.0) (`SpringArmComponent.TargetArmLength` _springarm_3)) 700.0 2200.0) _springarm_3)))
      (else
        (`SceneComponent.K2_SetRelativeRotation` _springarm (`KismetMathLibrary.MakeRotator` 0.0 (`KismetMathLibrary.FClamp` (+ _relativerotation_pitch (* (* (`self.Zoom`) -1.0) 10.0)) (`self.ZoomMin`) (`self.ZoomMax`))) false false)))))

(event `EnhancedInput|/Game/Main/Blueprints/PlayerController/Inputs/Inputs/Default/IA_Click`
  (params (ActionValue :type Boolean) (ElapsedSeconds :type "Float (double-precision)") (TriggeredSeconds :type "Float (double-precision)") (InputAction :type "InputAction Object Reference" :default "/Game/Main/Blueprints/PlayerController/Inputs/Inputs/Default/IA_Click.IA_Click"))
  (bind _returnvalue (subsystem `EnhancedInputLocalPlayerSubsystem`))
  (bind _army (`self.Army`))
  (bind (_hitresult _returnvalue_2) (`self.GetHitResultUnderCursorForObjects` (`|MakeArray` (cast `EObjectTypeQuery` 6))))
  (:`Completed`
    (if _returnvalue_2
      (bind _selected_unit (message `/Game/Main/Blueprints/Units/Interface/BPI_Unit.Selected` (`AIBlueprintHelperLibrary.GetAIController` (`.HitActor` (`GameplayStatics.BreakHitResult` _hitresult)))))
      (`KismetArrayLibrary.Array_AddUnique` _army _selected_unit)
      (`EnhancedInputSubsystemInterface.AddMappingContext` _returnvalue "/Game/Main/Blueprints/PlayerController/Inputs/IMC/Order/IMC_Order.IMC_Order" 0 (struct))
      (`KismetSystemLibrary.PrintText` (`|FormatText` "Selected : {Value}" (`KismetTextLibrary.Conv_ObjectToText` _selected_unit)) true true (struct :`G` 0.013418 :`B` 1.0 :`A` 1.0))
      (else
        (`KismetArrayLibrary.Array_Clear` _army)
        (`EnhancedInputSubsystemInterface.RemoveMappingContext` _returnvalue "/Game/Main/Blueprints/PlayerController/Inputs/IMC/Order/IMC_Order.IMC_Order" (struct))))))

(event `EnhancedInput|/Game/Main/Blueprints/PlayerController/Inputs/Inputs/Order/IA_GiveOrder`
  (params (ActionValue :type Boolean) (ElapsedSeconds :type "Float (double-precision)") (TriggeredSeconds :type "Float (double-precision)") (InputAction :type "InputAction Object Reference" :default "/Game/Main/Blueprints/PlayerController/Inputs/Inputs/Order/IA_GiveOrder.IA_GiveOrder"))
  (bind (_bblockinghit _binitialoverlap _time _distance _location) (`GameplayStatics.BreakHitResult` (`self.GetHitResultUnderCursorByChannel` "TraceTypeQuery1")))
  (:`Triggered`
    (for (_array_element _array_index) (`self.Army`)
      (message `/Game/Main/Blueprints/Units/Interface/BPI_Unit.CancelAction` _array_element false)
      (bind _returnvalue (`self.K2_GetPawn` _array_element))
      (bind _returnvalue_2 (`KismetMathLibrary.GetDirectionUnitVector` (`self.K2_GetActorLocation` _returnvalue) (+ (`KismetMathLibrary.MakeVector` (`KismetMathLibrary.Conv_IntToDouble` (* (/ _array_index 2) 150)) (`KismetMathLibrary.Conv_IntToDouble` (* (mod _array_index 2) 150))) _location)))
      (`Pawn.AddMovementInput` _returnvalue _returnvalue_2 1.0 false)
      (`self.K2_SetActorRotation` _returnvalue (`KismetMathLibrary.FindLookAtRotation` _returnvalue_2 _location) false)))
  (:`Completed`
    (for (_array_element_2 _array_index_2) (`self.Army`)
      (message `/Game/Main/Blueprints/Units/Interface/BPI_Unit.CancelAction` _array_element_2 true)
      (`/Game/Main/Blueprints/Units/AIController/AIC_Unit.MoveTo` _array_element_2 (+ (`KismetMathLibrary.MakeVector` (`KismetMathLibrary.Conv_IntToDouble` (* (/ _array_index_2 2) 150)) (`KismetMathLibrary.Conv_IntToDouble` (* (mod _array_index_2 2) 150))) (`.Location` (`GameplayStatics.BreakHitResult` (`self.GetHitResultUnderCursorByChannel` "TraceTypeQuery1"))))))))

(fn `UserConstructionScript`)